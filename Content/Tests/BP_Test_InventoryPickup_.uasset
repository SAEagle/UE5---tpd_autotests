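; Test pickup Blueprint for exercising the passing of data into an inventory pickup actor.
; SetInventoryData stores the inventory data and a color, then calls Init, which is not defined in this Blueprint.
; GenerateColor returns that stored test color.
; SetTestData prints its integer, float, string, boolean and vector inputs to verify received values.
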(event Custom|SetTestData
  (params (Int :type Integer) (Float :type Float%20%28double-precision%29) (Str :type String) (Bool :type Boolean) (Vec :type Vector))
  (Development|PrintString (Utilities|String|ToString(Integer) Int) true true "(R=0.000000,G=0.660000,B=1.000000,A=1.000000)" 1e+01)
  (Development|PrintString (Utilities|String|ToString(Float) Float) true true "(R=0.000000,G=0.660000,B=1.000000,A=1.000000)" 1e+01)
  (Development|PrintString Str true true "(R=0.000000,G=0.660000,B=1.000000,A=1.000000)" 1e+01)
  (Development|PrintString (Utilities|String|ToString(Boolean) Bool) true true "(R=0.000000,G=0.660000,B=1.000000,A=1.000000)" 1e+01)
  (Development|PrintString (Utilities|String|ToString(Vector) Vec) true true "(R=0.000000,G=0.660000,B=1.000000,A=1.000000)" 1e+01))

(event Custom|SetInventoryData
  (params (InvData :type Inventory%20Data%20Structure) (Color :type Linear%20Color%20Structure))
  (Variables|Default|SetInventoryData InvData)
  (Variables|Default|SetTestColor Color)
  (CallFunction|Init))

(event EventBeginPlay
  (|CallParentFunction) ; This node is disabled and will not be called.\nDrag off pins to build functionality.
)

(event Collision|EventActorBeginOverlap
  (params (OtherActor :type Actor%20Object%20Reference))
  (|CallParentFunction OtherActor) ; This node is disabled and will not be called.\nDrag off pins to build functionality.
)

(event EventTick
  (params (DeltaSeconds :type Float%20%28single-precision%29))
  (|CallParentFunction DeltaSeconds) ; This node is disabled and will not be called.\nDrag off pins to build functionality.
)

(fn ConstructionScript
  (|CallParentFunction))

(fn GenerateColor
  (return (Variables|Default|GetTestColor)))